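; BP_RecordingActor displays a swappable static mesh that the player can rotate for object inspection.
; SetNewMesh assigns the mesh and resets its transform, then UpdateScale fits it uniformly within DesiredExtend and offsets it by its bounds origin to recenter it.
; Rotation comes from click-drag mouse events or, while IsInspecting, from turn and look-up rates polled from BP_FirstPersonCharacter every Tick.
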(event `ClickedStart`
  (params (MouseLocation :type "Vector2D Structure"))
  (set `self.StartLocation` MouseLocation)
  (set `self.CanRotate` true))

(event `ClickedEnd`
  (set `self.CanRotate` false))

(event `MouseMove`
  (params (MouseLocation :type "Vector2D Structure"))
  (bind (_x _y) (`KismetMathLibrary.BreakVector2D` (- MouseLocation (`self.StartLocation`))))
  (if (`self.CanRotate`)
    (`SceneComponent.K2_AddWorldRotation` (`self.StaticMesh`) (`KismetMathLibrary.MakeRotator` 0.0 (* _y 0.5) (* _x -0.5)) false false)
    (set `self.StartLocation` MouseLocation)))

(event `UpdateScale`
  (bind _staticmesh (`self.StaticMesh`))
  (bind _staticmesh_2 (`self.StaticMesh`))
  (set `self.CurrentExtendMesh` (`.BoxExtent` (`KismetSystemLibrary.GetComponentBounds` (`self.StaticMesh`))))
  (`SceneComponent.SetWorldScale3D` _staticmesh (* (`SceneComponent.K2_GetComponentScale` _staticmesh) (`KismetMathLibrary.FMin` (/ (.x (`self.DesiredExtend`)) (.x (`self.CurrentExtendMesh`))) (/ (.y (`self.DesiredExtend`)) (.y (`self.CurrentExtendMesh`))) (/ (.z (`self.DesiredExtend`)) (.z (`self.CurrentExtendMesh`))))))
  (`SceneComponent.K2_AddLocalOffset` _staticmesh_2 (- (`SceneComponent.K2_GetComponentLocation` _staticmesh_2) (`KismetSystemLibrary.GetComponentBounds` _staticmesh_2)) false false))

(event `self.ReceiveBeginPlay`)

(event `GetCharacter`
  (bind _asbp_first_person_character (cast `/Game/ThirdPersonBP/Blueprints/BP_FirstPersonCharacter` (`GameplayStatics.GetPlayerCharacter` 0)))
  (bind _output_get (set `self.FirstPerson` _asbp_first_person_character))
  (set `self.LookUpRate` (`/Game/ThirdPersonBP/Blueprints/BP_FirstPersonCharacter.LookUpRate` _output_get))
  (set `self.TurnRate` (`/Game/ThirdPersonBP/Blueprints/BP_FirstPersonCharacter.TurnRate` _output_get))
  (set `self.IsInspecting?` (`/Game/ThirdPersonBP/Blueprints/BP_FirstPersonCharacter.IsInspecting?` _output_get)))

(event `self.ReceiveTick`
  (params (DeltaSeconds :type "Float (single-precision)"))
  (`|ExecutionSequence`
    (:`then_0`
      (`self.GetCharacter`))
    (:`then_1`
      (`self.TurnInspection`)
      (`self.LookUpInspection`))))

(fn `LookUpInspection`
  (if (`self.IsInspecting?`)
    (`SceneComponent.K2_AddWorldRotation` (`self.StaticMesh`) (`KismetMathLibrary.MakeRotator` 0.0 (* (`self.LookUpRate`) 4.0)) false false)))

(fn `SetNewMesh`
  (params (NewMesh :type "StaticMesh Object Reference"))
  (bind _staticmesh (`self.StaticMesh`))
  (`StaticMeshComponent.SetStaticMesh` _staticmesh NewMesh)
  (`SceneComponent.K2_SetRelativeLocation` _staticmesh (0.0 0.0 0.0) false false)
  (`SceneComponent.K2_SetRelativeRotation` :`self` _staticmesh)
  (`self.UpdateScale`))

(fn `TurnInspection`
  (if (`self.IsInspecting?`)
    (`SceneComponent.K2_AddWorldRotation` (`self.StaticMesh`) (`KismetMathLibrary.MakeRotator` 0.0 0.0 (* (`self.TurnRate`) -4.0)) false false)))

(fn `UserConstructionScript`)