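; Item inspection actor that displays a swappable static mesh and lets it be rotated with mouse movement.
; SetNewMesh resets the mesh transform, then UpdateScale fits it uniformly within DesiredExtend and offsets it to center its bounds.
; MouseMove turns cursor deltas into world pitch and yaw once ClickedStart enables rotation; ClickedEnd also leaves it enabled.
; Gamepad axis events and their turn functions are disconnected and do nothing.
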(event `InputAxis|TurnRate`
  (params (AxisValue :type "Float (single-precision)"))
  ;[1 1 1] Gamepad
)

(event `InputAxis|LookUpRate`
  (params (AxisValue :type "Float (single-precision)"))
  ;[1 1 1] Gamepad
)

(event `ClickedStart`
  (params (MouseLocation :type "Vector2D Structure"))
  (set `self.StartLocation` MouseLocation)
  (set `self.CanRotate` true))

(event `ClickedEnd`
  (set `self.CanRotate` true))

(event `MouseMove`
  (params (MouseLocation :type "Vector2D Structure"))
  (bind (_x _y) (`KismetMathLibrary.BreakVector2D` (- MouseLocation (`self.StartLocation`))))
  (if (`self.CanRotate`)
    (`SceneComponent.K2_AddWorldRotation` (`self.StaticMesh`) (`KismetMathLibrary.MakeRotator` 0.0 (* _y 0.5) (* _x -0.5)) false false)
    (set `self.StartLocation` MouseLocation)))

(event `self.ReceiveTick`
  (params (DeltaSeconds :type "Float (single-precision)")))

(event `UpdateScale`
  (bind _staticmesh (`self.StaticMesh`))
  (bind _staticmesh_2 (`self.StaticMesh`))
  (set `self.CurrentExtendMesh` (`.BoxExtent` (`KismetSystemLibrary.GetComponentBounds` (`self.StaticMesh`))))
  (`SceneComponent.SetWorldScale3D` _staticmesh (* (`SceneComponent.K2_GetComponentScale` _staticmesh) (`KismetMathLibrary.FMin` (/ (.x (`self.DesiredExtend`)) (.x (`self.CurrentExtendMesh`))) (/ (.y (`self.DesiredExtend`)) (.y (`self.CurrentExtendMesh`))) (/ (.z (`self.DesiredExtend`)) (.z (`self.CurrentExtendMesh`))))))
  (`SceneComponent.K2_AddLocalOffset` _staticmesh_2 (- (`SceneComponent.K2_GetComponentLocation` _staticmesh_2) (`KismetSystemLibrary.GetComponentBounds` _staticmesh_2)) false false))

(fn `SetNewMesh`
  (params (NewMesh :type "StaticMesh Object Reference"))
  (bind _staticmesh (`self.StaticMesh`))
  (`StaticMeshComponent.SetStaticMesh` _staticmesh NewMesh)
  (`SceneComponent.K2_SetRelativeLocation` _staticmesh (0.0 0.0 0.0) false false)
  (`SceneComponent.K2_SetRelativeRotation` :`self` _staticmesh)
  (`self.UpdateScale`))

(fn `TurnInspectionObject`
  (params (Value :type "Float (double-precision)")))

(fn `UpInspectionObject`
  (params (Value :type "Float (double-precision)")))

(fn `UserConstructionScript`
  (`parent.UserConstructionScript`))